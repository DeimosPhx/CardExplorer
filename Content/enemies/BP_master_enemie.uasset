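; Base enemy Blueprint that holds health, hit and death state, with a floating health bar.
; On BeginPlay it hands itself to the Floating_HB widget as its Enemy reference.
; TakeDmg subtracts from HP and sets the GetHit flag, or calls Die to zero HP and set IsDead when damage is lethal.
; DecideAction is a placeholder that returns zero.
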(event EventBeginPlay
  (bind _asfloating_hb (Utilities|Casting|CastToFloating_HB (UserInterface|GetUserWidgetObject (Variables|Default|GetHealthBar))))
  (Variables|/Game/UI/enemies/Floating_HB.Floating_HB_C|SetEnemy _asfloating_hb self))

(event Collision|EventActorBeginOverlap
  (params (OtherActor :type Actor%20Object%20Reference)))

(event EventTick
  (params (DeltaSeconds :type Float%20%28single-precision%29)))

(fn ConstructionScript)

(fn TakeDmg
  (params (DmgAmount :type Float%20%28single-precision%29))
  (if (<= (- (Variables|Default|GetHP) DmgAmount) 0.0)
    (Variables|Default|SetHP 0.0)
    (CallFunction|Die)
    (else
      (Variables|Default|SetHP (- (Variables|Default|GetHP) DmgAmount))
      (Variables|Default|SetgetHit true))))

(fn Die
  (Variables|Default|SetHP 0.0)
  (Variables|Default|SetisDead true))

(fn DecideAction
  (return 0.0))