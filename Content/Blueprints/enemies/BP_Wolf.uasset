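; BP_Wolf is a wolf enemy Blueprint that inherits its action choice, damage and death logic from a parent class.
; Its only added behavior is in TakeDmg, which calls the parent, then swaps the particle template for an impact effect on critical hits or a flash otherwise and activates it.
; DecideAction, Die and the construction script only forward to the parent, and the event graph is inactive.
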(event EventBeginPlay
  (|CallParentFunction) ; This node is disabled and will not be called.\nDrag off pins to build functionality.
)

(event Collision|EventActorBeginOverlap
  (params (OtherActor :type Actor%20Object%20Reference))
  (|CallParentFunction OtherActor) ; This node is disabled and will not be called.\nDrag off pins to build functionality.
)

(event EventTick
  (params (DeltaSeconds :type Float%20%28single-precision%29))
  (|CallParentFunction DeltaSeconds) ; This node is disabled and will not be called.\nDrag off pins to build functionality.
)

(fn ConstructionScript
  (|CallParentFunction))

(fn DecideAction
  (bind _dmgdealt (|CallParentFunction))
  (return _dmgdealt))

(fn TakeDmg
  (params (DmgAmount :type Float%20%28single-precision%29) (isCritical? :type Boolean))
  (bind _particlesystem (Variables|Default|GetParticleSystem))
  (|CallParentFunction DmgAmount isCritical?)
  (if isCritical?
    (Effects|Components|ParticleSystem|SetTemplate _particlesystem "/Game/AdvancedMagicFX13/Particles/P_ky_impact.P_ky_impact")
    (else
      (Effects|Components|ParticleSystem|SetTemplate _particlesystem "/Game/AdvancedMagicFX13/Particles/P_ky_flash1.P_ky_flash1")))
  (Components|Activation|Activate _particlesystem true))

(fn Die
  (|CallParentFunction))