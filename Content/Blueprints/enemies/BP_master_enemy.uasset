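; Base enemy Blueprint that handles health, damage, attacking, target marking and death.
; On BeginPlay it passes itself to its health bar and marker widgets.
; TakeDmg shows damage and critical hits on a widget, activates the hit sound, then lowers HP or calls Die, which reuses the attack audio component for the death sound.
; DecideAction simply flags attacking and returns the attack value, while other state is exposed as hit, dead and marked booleans.
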(event EventBeginPlay
  (bind _asfloating_hb (Utilities|Casting|CastToFloating_HB (UserInterface|GetUserWidgetObject (Variables|Default|GetHealthBar))))
  (Variables|/Game/UI/enemies/Floating_HB.Floating_HB_C|SetEnemy _asfloating_hb self)
  (Variables|Default|SetIsMarked? false)
  (bind _asmarker_wb (Utilities|Casting|CastToMarker_WB (UserInterface|GetUserWidgetObject (Variables|Default|GetMarker))))
  (Variables|/Game/UI/enemies/Marker_WB.Marker_WB_C|SetEnemy _asmarker_wb self))

(event Collision|EventActorBeginOverlap
  (params (OtherActor :type Actor%20Object%20Reference)))

(event EventTick
  (params (DeltaSeconds :type Float%20%28single-precision%29)))

(fn ConstructionScript)

(fn TakeDmg
  (params (DmgAmount :type Float%20%28single-precision%29) (isCritical? :type Boolean))
  (bind _asdamage_wb (Utilities|Casting|CastToDamage_WB (UserInterface|GetUserWidgetObject (Variables|Default|GetDmgWB)))
    (:then
      (Default|DisplayDamage _asdamage_wb DmgAmount isCritical?))
    (:CastFailed
      _))
  (Components|Activation|Activate (Variables|Default|GetHit_SC) true)
  (if (<= (- (Variables|Default|GetHP) DmgAmount) 0.0)
    (Variables|Default|SetHP 0.0)
    (CallFunction|Die)
    (else
      (Variables|Default|SetHP (- (Variables|Default|GetHP) DmgAmount))
      (Variables|Default|SetgetHit true))))

(fn Die
  (bind _atk_sc (Variables|Default|GetAtk_SC))
  (Components|Activation|Deactivate (Variables|Default|GetIdle_SC))
  (Audio|Components|Audio|SetSound _atk_sc (Variables|Default|GetDie_SC))
  (Components|Activation|Activate _atk_sc true)
  (Variables|Default|SetHP 0.0)
  (Variables|Default|SetisDead true))

(fn DecideAction
  (Variables|Default|SetisAttaking true)
  (return (Variables|Default|GetAtkValue)))

(fn MarkEnemy
  (params (Show? :type Boolean))
  (Variables|Default|SetIsMarked? Show?))