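; Base actor for selectable entries in the main menu, each with a configurable title and a widget to open.
; On BeginPlay it copies MenuTitle into the Main_menu_selector_title widget hosted by its Title component.
; Its IsSelected event creates the WidgetToShow widget, adds it to the viewport and clears CanSelectMainMenuSelector on the Adventurer_PC player controller to block further selection.
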(event Custom|IsSelected
  (bind _returnvalue (UserInterface|CreateWidget (Variables|Default|GetwidgetToShow)))
  (UserInterface|Viewport|AddtoViewport _returnvalue 0)
  (bind _asadventurer_pc (Utilities|Casting|CastToAdventurer_PC (Game|GetPlayerController 0)))
  (Variables|/Game/Adventurer_PC.Adventurer_PC_C|SetCanSelectMainMenuSelector? _asadventurer_pc false))

(event EventBeginPlay
  (bind _asmain_menu_selector_title (Utilities|Casting|CastToMain_menu_selector_title (UserInterface|GetUserWidgetObject (Variables|Default|Gettitle))))
  (Variables|/Game/UI/main_menu/Main_menu_selector_title.Main_menu_selector_title_C|Setcontext_title _asmain_menu_selector_title (Variables|Default|Getmenu_title)))

(event Collision|EventActorBeginOverlap
  (params (OtherActor :type Actor%20Object%20Reference)))

(event EventTick
  (params (DeltaSeconds :type Float%20%28single-precision%29)))

(fn ConstructionScript)